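; Player controller that routes player input to the possessed Character_BP and handles the pause menu.
; It caches the character on possess, then forwards interact, dash and world-axis movement inputs to it.
; Any key press checks for a gamepad key and signals when the device type changes.
; TogglePause creates or removes the pause widget, switching input mode, cursor visibility and game pause state.
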(event `Key|AnyKey`
  (params (Key :type "Key Structure"))
  (bind _returnvalue (`KismetInputLibrary.Key_IsGamepadKey` Key))
  (:`Pressed`
    (if (!= _returnvalue (`self.bIsUsingGamepad`))
      (`self.GamepadChanged` _returnvalue))))

(event `InputAction|Drop`
  (params (Key :type "Key Structure")))

(event `InputAction|Interact`
  (params (Key :type "Key Structure"))
  (:`Pressed`
    (`/Game/Blueprints/Character/Character_BP.Interact` (`self.PlayerChara`))))

(event `InputAction|Pause` :paused true
  (params (Key :type "Key Structure"))
  (:`Pressed`
    (`self.TogglePause`)))

(event `InputAction|Dash`
  (params (Key :type "Key Structure"))
  (:`Pressed`
    (bind _playerchara (`self.PlayerChara`)
      (:`then`
        (`/Game/Blueprints/Character/Character_BP.Dash` _playerchara))
      (:`else`))))

(event `InputAxis|MoveRight`
  (params (AxisValue :type "Float (single-precision)"))
  (bind _playerchara (`self.PlayerChara`)
    (:`then`
      (`/Game/Blueprints/Character/Character_BP.AddInputMovement` _playerchara (0.0 1.0 0.0) AxisValue false))
    (:`else`)))

(event `InputAxis|MoveUp`
  (params (AxisValue :type "Float (single-precision)"))
  (bind _playerchara (`self.PlayerChara`)
    (:`then`
      (`/Game/Blueprints/Character/Character_BP.AddInputMovement` _playerchara (1.0 0.0 0.0) AxisValue false))
    (:`else`)))

(event `self.ReceivePossess`
  (params (PossessedPawn :type "Pawn Object Reference"))
  (bind _ascharacter_bp (cast `/Game/Blueprints/Character/Character_BP` PossessedPawn))
  (set `self.PlayerChara` _ascharacter_bp))

(fn `TogglePause`
  (bind _returnvalue (not (`GameplayStatics.IsGamePaused`)))
  (if (`GameplayStatics.IsGamePaused`)
    (`Widget.RemoveFromParent` (`self.PauseWidget`))
    (`WidgetBlueprintLibrary.SetInputMode_GameOnly` self)
    (else
      (bind _returnvalue_2 (`|CreateWidget` "/Game/Blueprints/UI/Pause_Widget.Pause_Widget_C" self))
      (bind _output_get (set `self.PauseWidget` _returnvalue_2))
      (`UserWidget.AddToViewport` _output_get 0)
      (`WidgetBlueprintLibrary.SetInputMode_UIOnlyEx` self _output_get)))
  (set `self.bShowMouseCursor` _returnvalue)
  (`GameplayStatics.SetGamePaused` _returnvalue))

(fn `UserConstructionScript`)