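; EnemyCharacter_BP is a patrolling enemy that stuns any other Character_BP overlapping its capsule.
; On BeginPlay it starts an AI MoveTo loop through the PatrolPath actors, advancing the index on each arrival and wrapping to the first.
; A failed move only prints "Fail" and ends the patrol.
; The capsule overlap casts to Character_BP, excludes itself, and calls Stun on the other character.
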(event `self.ReceiveBeginPlay`
  (`parent.ReceiveBeginPlay`)
  (`|AIMoveTo` self (0.0 0.0 0.0) (`|GetArrayItem` (`self.PatrolPath`) (`self.CurrentPatrolIndex`)) :!label _label
    (:`OnSuccess`
      (bind _result (`/Engine/EditorBlueprintResources/StandardMacros.IncrementInt` (`self.CurrentPatrolIndex`))
        (:`  `
          (if (== _result (`KismetArrayLibrary.Array_Length` (`self.PatrolPath`)))
            (set `self.CurrentPatrolIndex` 0)
            (goto _label)
            (else
              (goto _label))))))
    (:`OnFail`
      (`KismetSystemLibrary.PrintString` "Fail"))))

(event `self.Capsule.OnComponentBeginOverlap`
  (params (OverlappedComponent :type "PrimitiveComponent Object Reference") (OtherActor :type "Actor Object Reference") (OtherComp :type "PrimitiveComponent Object Reference") (OtherBodyIndex :type Integer) (bFromSweep :type Boolean) (SweepResult :type "HitResult Structure (by ref)"))
  (bind _ascharacter_bp (cast `/Game/Blueprints/Character/Character_BP` OtherActor))
  (if (!= _ascharacter_bp self)
    (`self.Stun` _ascharacter_bp)))

(fn `UserConstructionScript`
  (`parent.UserConstructionScript`))