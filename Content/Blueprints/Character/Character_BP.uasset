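; Playable character Blueprint with dashing, stun, slow, carrying one object and interacting with Interactible actors.
; Tick applies accumulated input, turns the controller toward movement and sphere-traces ahead to update interaction focus.
; Dash adds an impulse along last input; a hit mid-dash stuns the character, with timed recovery and invulnerability, through event dispatchers.
; Held objects attach to a mesh socket, and slowing lowers walk speed and blocks dashing.
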(event `self.ReceiveBeginPlay`
  (add `self.OnStun` (`|CreateDelegate` :!event `OnStun_`))
  (add `self.OnDashHitWall` (`|CreateDelegate` :!event `OnDashHitWall_Event`))
  (add `self.OnDash` (`|CreateDelegate` :!event `OnDash_Event`)))

(event `self.ReceiveTick`
  (params (DeltaSeconds :type "Float (single-precision)"))
  (`self.LookAtMoveDirection` DeltaSeconds)
  (`PawnMovementComponent.AddInputVector` (`self.CharacterMovement`) (`self.InputMovement`) false)
  (set `self.InputMovement` (0.0 0.0 0.0))
  (`self.UpdateInteraction`))

(event `OnStun_`
  (`|ExecutionSequence`
    (:`then_0`
      (`KismetSystemLibrary.Delay` (`self.StunRecoveryDelay`))
      (set `self.bIsStun` false))
    (:`then_1`
      (`KismetSystemLibrary.Delay` (`self.InvulnerabilityDurationAfterStun`))
      (set `self.bInvulnerable` false))))

(event `self.ReceiveHit`
  (params (MyComp :type "PrimitiveComponent Object Reference") (Other :type "Actor Object Reference") (OtherComp :type "PrimitiveComponent Object Reference") (bSelfMoved :type Boolean) (HitLocation :type "Vector Structure") (HitNormal :type "Vector Structure") (NormalImpulse :type "Vector Structure") (Hit :type "HitResult Structure (by ref)"))
  (if (and (`self.bIsDashing`) (not (`self.bInvulnerable`)))
    (`self.OnDashHitWall`)))

(event `OnDashHitWall_Event`
  (`self.Stun`)
  (`GameplayStatics.PlaySound2D` "/Game/Sounds/Hit.Hit" 1.0 1.0 0.0 null null))

(event `OnDash_Event`
  (`GameplayStatics.PlaySound2D` "/Game/Sounds/Dash.Dash" 1.0 1.0 0.0 null null)
  (`KismetSystemLibrary.Delay` (`self.DashDuration`))
  (set `self.bIsDashing` false))

(event `self.SetObject`
  (params (Object :type "/Game/Blueprints/Interactions/Ingredients_BP Object Reference"))
  (bind _output_get (set `self.ObjectInHand` Object))
  (`self.K2_AttachToComponent` _output_get (`self.Mesh`) "Object_Socket" "SnapToTarget" "SnapToTarget" "KeepWorld" true))

(event `self.ClearObject`
  (bind _objectinhand (`self.ObjectInHand`))
  (`/Engine/EditorBlueprintResources/StandardMacros.IsValid` _objectinhand
    (:`Is Valid`
      (`self.K2_DetachFromActor` _objectinhand "KeepWorld" "KeepWorld" "KeepWorld")
      (set `self.ObjectInHand` null))))

(fn `AddInputMovement`
  (params (WorldDirection :type "Vector Structure") (ScaleValue :type "Float (double-precision)") (bForce :type Boolean))
  (if (not (`self.bIsStun`))
    (set `self.InputMovement` (+ (* (`KismetMathLibrary.Normal` WorldDirection) ScaleValue) (`self.InputMovement`)))))

(fn `Dash`
  (if (not (or (`self.bIsStun`) (`self.bIsSlowed`)))
    (`CharacterMovementComponent.AddImpulse` (`self.CharacterMovement`) (* (`KismetMathLibrary.Normal` (`PawnMovementComponent.GetLastInputVector` (`self.CharacterMovement`))) (`self.DashStrength`)) true)
    (set `self.bIsDashing` true)
    (`self.OnDash`)))

(fn `GetObject`
  (returns (ObjectInHand :type "/Game/Blueprints/Interactions/Ingredients_BP Object Reference"))
  (return (`self.ObjectInHand`)))

(fn `HasSomethingInHands`
  (returns (HasSomething :type Boolean))
  (return (`KismetSystemLibrary.IsValid` (`self.ObjectInHand`))))

(fn `Interact`
  (`/Engine/EditorBlueprintResources/StandardMacros.IsValid` (`KismetSystemLibrary.Conv_InterfaceToObject` (`self.InteractionFocus`))
    (:`Is Valid`
      (`/Game/Blueprints/Interactions/Interactible.Interact` (`self.InteractionFocus`) self))))

(fn `IsStuned`
  (returns (Stuned :type Boolean))
  (return (`self.bIsStun`)))

(fn `LookAtMoveDirection`
  (params (DeltaTime :type "Float (double-precision)"))
  (bind _returnvalue (`self.GetController`))
  (bind _returnvalue_2 (`self.K2_GetActorLocation`))
  (if (!= (`self.InputMovement`) (0.0 0.0 0.0))
    (`Controller.SetControlRotation` _returnvalue (`KismetMathLibrary.RInterpTo` (`Controller.GetControlRotation` _returnvalue) (`KismetMathLibrary.FindLookAtRotation` _returnvalue_2 (+ _returnvalue_2 (`self.InputMovement`))) DeltaTime (`self.RotationSpeed`)))))

(fn `StartSlow`
  (bind _charactermovement (`self.CharacterMovement`))
  (set `CharacterMovementComponent.MaxWalkSpeed` (`self.SlowedSpeed`) _charactermovement)
  (set `self.bIsSlowed` true)
  (`MovementComponent.StopMovementImmediately` _charactermovement))

(fn `StopSlow`
  (set `CharacterMovementComponent.MaxWalkSpeed` 600.0 (`self.CharacterMovement`))
  (set `self.bIsSlowed` false))

(fn `Stun`
  (if (not (`self.bInvulnerable`))
    (set `self.bIsStun` true)
    (set `self.bInvulnerable` true)
    (`KismetSystemLibrary.PrintString` "Stuned ! " true true (struct :`R` 1.0 :`A` 1.0))
    (`self.OnStun`)))

(fn `TakeObjectInHand`
  (returns (Ingredient :type "/Game/Blueprints/Interactions/Ingredients_BP Object Reference"))
  (locals (Object :type "/Game/Blueprints/Interactions/Ingredients_BP Object Reference"))
  (bind _objectinhand (`self.ObjectInHand`)
    (:`then`
      (bind _output_get (set `local.Object` _objectinhand))
      (`self.ClearObject`)
      (return _output_get))
    (:`else`
      (return null))))

(fn `UpdateInteraction`
  (locals (NewLocalVar_0 :type "Array of EObjectTypeQuery Enum"))
  (bind _returnvalue (`self.K2_GetActorLocation`))
  (bind _returnvalue_2 (`KismetSystemLibrary.Conv_InterfaceToObject` (`self.InteractionFocus`)))
  (bind _outhits (`KismetSystemLibrary.SphereTraceMulti` :`Start` _returnvalue :`End` (+ _returnvalue (* (`self.GetActorForwardVector`) (`self.InteractionCheckDistance`))) :`Radius` (`self.InteractionCheckRadius`) :`TraceChannel` "TraceTypeQuery3" :`DrawTime` 0.0))
  (for _array_element _outhits
    (bind _asinteractible (cast `/Game/Blueprints/Interactions/Interactible` (`.HitActor` (`GameplayStatics.BreakHitResult` _array_element))))
    (bind _caninteract (`/Game/Blueprints/Interactions/Interactible.CanInteract` _asinteractible self))
    (if _caninteract
      (if (!= _returnvalue_2 (`.HitActor` (`GameplayStatics.BreakHitResult` _array_element)))
        (`/Engine/EditorBlueprintResources/StandardMacros.IsValid` _returnvalue_2
          (:`Is Valid`
            (`/Game/Blueprints/Interactions/Interactible.LooseFocus` (`self.InteractionFocus`)))
          (:`Is Not Valid`
            _))
        (bind _output_get (set `self.InteractionFocus` _asinteractible))
        (`/Game/Blueprints/Interactions/Interactible.GainFocus` _output_get)
        (return)
        (else
          (return)))))
  (`/Engine/EditorBlueprintResources/StandardMacros.IsValid` (`KismetSystemLibrary.Conv_InterfaceToObject` (`self.InteractionFocus`))
    (:`Is Valid`
      (`/Game/Blueprints/Interactions/Interactible.LooseFocus` (`self.InteractionFocus`))
      (set `self.InteractionFocus` null))))

(fn `UserConstructionScript`)