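; Mixer interactable that collects a required set of ingredients from players carrying objects.
; Interact takes and destroys the held object, ticking its class off a class-to-bool map and broadcasting OnGoodIngredient, or stunning the player if it is unlisted or already added.
; IsFull reports when every ingredient is in, and GetScoreTime rates elapsed time from 3 to 0 against gold, silver and bronze thresholds.
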(event `/Game/Blueprints/Interactions/Interactible.Interact`
  (params (Player :type "/Game/Blueprints/Character/Character_BP Object Reference"))
  (bind _ingredient (`/Game/Blueprints/Character/Character_BP.TakeObjectInHand` Player))
  (bind _returnvalue (`GameplayStatics.GetObjectClass` _ingredient))
  (bind (_value _returnvalue_2) (`BlueprintMapLibrary.Map_Find` (`self.IngredientRequiredList`) _returnvalue))
  (if _returnvalue_2
    (if _value
      (`/Game/Blueprints/Character/Character_BP.Stun` Player :!label _label)
      (else
        (`BlueprintMapLibrary.Map_Add` (`self.IngredientRequiredList`) _returnvalue true)
        (`self.OnGoodIngredient` _returnvalue)))
    (else
      (goto _label)))
  (`self.K2_DestroyActor` _ingredient))

(event `/Game/Blueprints/ObjectHolder.ClearObject`)

(event `/Game/Blueprints/ObjectHolder.SetObject`
  (params (Object :type "/Game/Blueprints/Interactions/Ingredients_BP Object Reference")))

(fn `CanInteract`
  (params (Player :type "/Game/Blueprints/Character/Character_BP Object Reference"))
  (returns (CanInteract :type Boolean))
  (return (`/Game/Blueprints/Character/Character_BP.HasSomethingInHands` Player)))

(fn `GetScoreTime`
  (params (TimeElapsed :type "Float (double-precision)"))
  (returns (Score :type Integer))
  (if (<= TimeElapsed (`self.GoldTime`))
    (return 3)
    (elif (<= TimeElapsed (`self.SilverTime`))
      (return 2)
      (elif (<= TimeElapsed (`self.BronzeTime`))
        (return 1)
        (else
          (return 0))))))

(fn `IsFull`
  (returns (`Full?` :type Boolean))
  (bind _keys (`BlueprintMapLibrary.Map_Keys` (`self.IngredientRequiredList`)))
  (for _array_element _keys
    (if (not (`BlueprintMapLibrary.Map_Find` (`self.IngredientRequiredList`) _array_element))
      (return false)))
  (return true))

(fn `UserConstructionScript`)