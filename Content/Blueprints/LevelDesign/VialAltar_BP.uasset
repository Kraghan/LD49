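; Vial altar level object that keeps an ingredient of a configurable class at its item position.
; It spawns the ingredient on BeginPlay and makes itself the owner.
; When ClearObject fires, it runs the parent logic and spawns a replacement, acting as a self-refilling dispenser.
; CanInteract always returns false, so the altar itself rejects player interaction.
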(event `self.ReceiveBeginPlay`
  (`self.SpawnIngredient`))

(event `/Game/Blueprints/ObjectHolder.ClearObject`
  (`parent.ClearObject`)
  (`self.SpawnIngredient`))

(fn `CanInteract`
  (params (Player :type "/Game/Blueprints/Character/Character_BP Object Reference"))
  (returns (CanInteract :type Boolean))
  (return false))

(fn `SpawnIngredient`
  (bind _returnvalue (`|SpawnActorFromClass` (`self.IngredientToSpawn`) (`KismetMathLibrary.MakeTransform` (`SceneComponent.K2_GetComponentLocation` (`self.ItemPosition`))) "AdjustIfPossibleButAlwaysSpawn" "OverrideRootScale" null null))
  (`/Game/Blueprints/Interactions/Ingredients_BP.ChangeOwner` _returnvalue self))

(fn `UserConstructionScript`)