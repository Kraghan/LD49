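; Block_BP is an interactable pedestal where the player places a held item, available only when hands are full and the block is empty.
; Interact takes the player's object, makes the block its owner and plays a placing sound.
; SetObject stores the object and snaps it to ItemPosition, while ClearObject empties the slot.
; A billboard prompt appears on focus and swaps between keyboard and Xbox icons through the player controller's gamepad event.
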(event `self.ReceiveBeginPlay`
  (bind _asplayer_controller_bp (cast `/Game/Blueprints/Character/PlayerController_BP` (`GameplayStatics.GetPlayerController` 0)))
  (add `/Game/Blueprints/Character/PlayerController_BP.GamepadEvent` _asplayer_controller_bp (delegate `GamepadChanged`)))

(event `GamepadChanged`
  (params (GamepadActive :type Boolean))
  (bind _billboard (`self.Billboard`))
  (if GamepadActive
    (`BillboardComponent.SetSprite` _billboard "/Game/Textures/UI/UI_menuNEW/a_xbox_black.a_xbox_black")
    (else
      (`BillboardComponent.SetSprite` _billboard "/Game/Textures/UI/UI_menuNEW/e_key_black.e_key_black"))))

(event `/Game/Blueprints/Interactions/Interactible.Interact`
  (params (Player :type "/Game/Blueprints/Character/Character_BP Object Reference"))
  (bind _ingredient (`/Game/Blueprints/Character/Character_BP.TakeObjectInHand` Player))
  (`/Game/Blueprints/Interactions/Ingredients_BP.ChangeOwner` _ingredient self)
  (`GameplayStatics.PlaySound2D` "/Game/Sounds/Flask_Poser_Cue.Flask_Poser_Cue" 2.0 1.0 0.0 null null))

(event `/Game/Blueprints/ObjectHolder.SetObject`
  (params (Object :type "/Game/Blueprints/Interactions/Ingredients_BP Object Reference"))
  (bind _output_get (set `self.ObjectOnIt` Object))
  (`self.K2_SetActorLocation` _output_get (`SceneComponent.K2_GetComponentLocation` (`self.ItemPosition`)) false true)
  (`self.K2_SetActorRotation` _output_get (`SceneComponent.K2_GetComponentRotation` (`self.ItemPosition`)) true))

(event `/Game/Blueprints/ObjectHolder.ClearObject`
  (set `self.ObjectOnIt` null))

(event `/Game/Blueprints/Interactions/Interactible.GainFocus`
  (`SceneComponent.SetHiddenInGame` (`self.Billboard`) false false))

(event `/Game/Blueprints/Interactions/Interactible.LooseFocus`
  (`SceneComponent.SetHiddenInGame` (`self.Billboard`) true false))

(fn `CanInteract`
  (params (Player :type "/Game/Blueprints/Character/Character_BP Object Reference"))
  (returns (CanInteract :type Boolean))
  (return (and (`/Game/Blueprints/Character/Character_BP.HasSomethingInHands` Player) (not (`KismetSystemLibrary.IsValid` (`self.ObjectOnIt`))))))

(fn `UserConstructionScript`)