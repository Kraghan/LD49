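; Puddle actor that slows a Character_BP while it overlaps the puddle's sphere.
; Sphere begin and end overlap events call StartSlow and StopSlow on the character.
; Unless LifeTime is zero or less, it waits that long after BeginPlay, then a timeline animates its scale relative to the current size and destroys it when finished.
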(event `self.ReceiveBeginPlay`
  (if (not (<= (`self.LifeTime`) 0.0))
    (`KismetSystemLibrary.Delay` (`self.LifeTime`))
    (set `self.BaseScale` (`self.GetActorScale3D`))
    (bind (_direction _scale) (`Timeline|Scale` :!via `PlayFromStart`)
      (:`Update`
        (`self.SetActorScale3D` (* (`self.BaseScale`) _scale)))
      (:`Finished`
        (`self.K2_DestroyActor`)))))

(event `self.Sphere.OnComponentBeginOverlap`
  (params (OverlappedComponent :type "PrimitiveComponent Object Reference") (OtherActor :type "Actor Object Reference") (OtherComp :type "PrimitiveComponent Object Reference") (OtherBodyIndex :type Integer) (bFromSweep :type Boolean) (SweepResult :type "HitResult Structure (by ref)"))
  (bind _ascharacter_bp (cast `/Game/Blueprints/Character/Character_BP` OtherActor))
  (`/Game/Blueprints/Character/Character_BP.StartSlow` _ascharacter_bp))

(event `self.Sphere.OnComponentEndOverlap`
  (params (OverlappedComponent :type "PrimitiveComponent Object Reference") (OtherActor :type "Actor Object Reference") (OtherComp :type "PrimitiveComponent Object Reference") (OtherBodyIndex :type Integer))
  (bind _ascharacter_bp (cast `/Game/Blueprints/Character/Character_BP` OtherActor))
  (`/Game/Blueprints/Character/Character_BP.StopSlow` _ascharacter_bp))

(fn `UserConstructionScript`)