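; Interactable recipe actor that opens a full Recipe_Widget on screen when the player interacts with it.
; The widget is created collapsed at BeginPlay; Interact reveals it, switches to UI-only input with a visible cursor and plays a letter-reading sound.
; A billboard prompt shows on focus, hides on focus loss, and swaps between keyboard and Xbox icons through the player controller's gamepad event.
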(event `self.ReceiveBeginPlay`
  (`parent.ReceiveBeginPlay`)
  (bind _returnvalue (`|CreateWidget` "/Game/Blueprints/UI/Recipe_Widget.Recipe_Widget_C" (`GameplayStatics.GetPlayerController` 0)))
  (`UserWidget.AddToViewport` _returnvalue 0)
  (bind _output_get (set `self.UI` _returnvalue))
  (`Widget.SetVisibility` _output_get "Collapsed")
  (bind _asplayer_controller_bp (cast `/Game/Blueprints/Character/PlayerController_BP` (`GameplayStatics.GetPlayerController` 0)))
  (add `/Game/Blueprints/Character/PlayerController_BP.GamepadEvent` _asplayer_controller_bp (delegate `GamepadChanged`)))

(event `GamepadChanged`
  (params (GamepadActive :type Boolean))
  (bind _billboard (`self.Billboard`))
  (if GamepadActive
    (`BillboardComponent.SetSprite` _billboard "/Game/Textures/UI/UI_menuNEW/a_xbox_black.a_xbox_black")
    (else
      (`BillboardComponent.SetSprite` _billboard "/Game/Textures/UI/UI_menuNEW/e_key_black.e_key_black"))))

(event `self.ReceiveTick`
  (params (DeltaSeconds :type "Float (single-precision)"))
  (`parent.ReceiveTick` DeltaSeconds))

(event `/Game/Blueprints/Interactions/Interactible.GainFocus`
  (`SceneComponent.SetHiddenInGame` (`self.Billboard`) false false))

(event `/Game/Blueprints/Interactions/Interactible.LooseFocus`
  (`SceneComponent.SetHiddenInGame` (`self.Billboard`) true false))

(event `/Game/Blueprints/Interactions/Interactible.Interact`
  (params (Player :type "/Game/Blueprints/Character/Character_BP Object Reference"))
  (bind _returnvalue (`GameplayStatics.GetPlayerController` 0))
  (`Widget.SetVisibility` (`self.UI`) "Visible")
  (`WidgetBlueprintLibrary.SetInputMode_UIOnlyEx` _returnvalue null "LockOnCapture")
  (set `PlayerController.bShowMouseCursor` true _returnvalue)
  (`GameplayStatics.PlaySound2D` "/Game/Sounds/UISound_lire_la_lettre.UISound_lire_la_lettre" 1.0 1.0 0.0 null null))

(fn `CanInteract`
  (params (Player :type "/Game/Blueprints/Character/Character_BP Object Reference"))
  (returns (CanInteract :type Boolean))
  (return true))

(fn `UserConstructionScript`
  (`parent.UserConstructionScript`))