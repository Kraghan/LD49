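; Level-design hazard actor that periodically vents steam and stuns characters inside its capsule.
; Activate and Deactivate call each other after delays, toggling the steam effect and active flag in an endless timed cycle.
; Activation stuns Character_BP actors already overlapping, while the capsule's begin-overlap stuns those entering during the active phase.
; A start-enabled flag and start offset set the initial phase, so placed instances can be staggered.
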(event `self.ReceiveBeginPlay`
  (if (`self.bStartEnabled`)
    (`self.Activate` (- (`self.ActiveDuration`) (`self.StartOffset`)))
    (else
      (`self.Deactivate` (- (`self.DisableDuration`) (`self.StartOffset`))))))

(event `self.Capsule.OnComponentBeginOverlap`
  (params (OverlappedComponent :type "PrimitiveComponent Object Reference") (OtherActor :type "Actor Object Reference") (OtherComp :type "PrimitiveComponent Object Reference") (OtherBodyIndex :type Integer) (bFromSweep :type Boolean) (SweepResult :type "HitResult Structure (by ref)"))
  (if (`self.bIsActive`)
    (bind _ascharacter_bp (cast `/Game/Blueprints/Character/Character_BP` OtherActor))
    (`/Game/Blueprints/Character/Character_BP.Stun` _ascharacter_bp)))

(event `Activate`
  (params (ActivationDuration :type "Float (double-precision)"))
  (`ActorComponent.Activate` (`self.Steamfx`) true)
  (set `self.bIsActive` true)
  (for _array_element (`PrimitiveComponent.GetOverlappingActors` (`self.Capsule`) "/Game/Blueprints/Character/Character_BP.Character_BP_C")
    (bind _ascharacter_bp (cast `/Game/Blueprints/Character/Character_BP` _array_element))
    (`/Game/Blueprints/Character/Character_BP.Stun` _ascharacter_bp))
  (`KismetSystemLibrary.Delay` ActivationDuration)
  (`self.Deactivate` (`self.DisableDuration`)))

(event `Deactivate`
  (params (DeactivationDuration :type "Float (double-precision)"))
  (`ActorComponent.Deactivate` (`self.Steamfx`))
  (set `self.bIsActive` false)
  (`KismetSystemLibrary.Delay` DeactivationDuration)
  (`self.Activate` (`self.ActiveDuration`)))

(fn `UserConstructionScript`)