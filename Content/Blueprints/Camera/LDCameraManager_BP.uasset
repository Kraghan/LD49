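; Player camera manager that overrides BlueprintUpdateCamera to place the view at a stored 2D location with set height, rotation and FOV.
; The live update projects Character_BP to a screen ratio but never uses it, so it never moves the stored location.
; Unconnected nodes hold an unfinished follow: IsOutOfBounds clamps that ratio to hard and soft dead zones, then deprojection and VInterpTo smooth the camera toward the result.
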(event `self.ReceiveTick`
  (params (DeltaSeconds :type "Float (single-precision)")))

(fn `BlueprintUpdateCamera`
  (params (CameraTarget :type "Actor Object Reference"))
  (returns (NewCameraLocation :type "Vector Structure") (NewCameraRotation :type "Rotator Structure") (NewCameraFOV :type "Float (double-precision)") (ReturnValue :type Boolean))
  (locals (PlayerScreenPosInRatio :type "Vector2D Structure") (NewLocation2D :type "Vector2D Structure") (PlayerScreenPos :type "Vector2D Structure") (bIsOutBounds :type Boolean))
  (bind (_currentcameralocation2d_x _currentcameralocation2d_y) (`KismetMathLibrary.BreakVector2D` (`self.CurrentCameraLocation2D`)))
  (bind _ascharacter_bp (cast `/Game/Blueprints/Character/Character_BP` (`GameplayStatics.GetPlayerPawn` 0)))
  (bind (_screenposition _returnvalue) (`GameplayStatics.ProjectWorldToScreen` (`self.GetOwningPlayerController`) (`self.K2_GetActorLocation` _ascharacter_bp)))
  (bind _output_get (set `local.PlayerScreenPos` _screenposition))
  (bind _output_get_2 (set `local.PlayerScreenPosInRatio` (/ _output_get (`WidgetLayoutLibrary.GetViewportSize`))))
  (if _returnvalue
    _
    (else
      _))
  (return (`KismetMathLibrary.MakeVector` _currentcameralocation2d_x _currentcameralocation2d_y (`self.CameraHeigth`)) (`self.CameraRotation`) (`self.FOV`) true))

(fn `IsOutOfBounds`
  (params (DeadZone :type "Vector2D Structure") (ScreenPos :type "Vector2D Structure"))
  (returns (bIsOutOfBound :type Boolean) (FinalPos :type "Vector2D Structure"))
  (locals (ResultPos :type "Vector2D Structure") (bIsOutBounds :type Boolean))
  (bind (_deadzone_x _deadzone_y) (`KismetMathLibrary.BreakVector2D` (`local.DeadZone`)))
  (bind _deadzone_x_2 (`KismetMathLibrary.BreakVector2D` (`local.DeadZone`)))
  (bind (_deadzone_x_3 _deadzone_y_2) (`KismetMathLibrary.BreakVector2D` (`local.DeadZone`)))
  (bind (_deadzone_x_4 _deadzone_y_3) (`KismetMathLibrary.BreakVector2D` (`local.DeadZone`)))
  (bind _deadzone_x_5 (`KismetMathLibrary.BreakVector2D` (`local.DeadZone`)))
  (bind _screenpos_x (`KismetMathLibrary.BreakVector2D` (`local.ScreenPos`)))
  (bind _screenpos_x_2 (`KismetMathLibrary.BreakVector2D` (`local.ScreenPos`)))
  (bind _resultpos_x (`KismetMathLibrary.BreakVector2D` (`local.ResultPos`)))
  (bind (_screenpos_x_3 _screenpos_y) (`KismetMathLibrary.BreakVector2D` (`local.ScreenPos`)))
  (bind _deadzone_x_6 (`KismetMathLibrary.BreakVector2D` (`local.DeadZone`)))
  (bind (_screenpos_x_4 _screenpos_y_2) (`KismetMathLibrary.BreakVector2D` (`local.ScreenPos`)))
  (bind _resultpos_x_2 (`KismetMathLibrary.BreakVector2D` (`local.ResultPos`)))
  (bind (_resultpos_x_3 _resultpos_y) (`KismetMathLibrary.BreakVector2D` (`local.ResultPos`)))
  (bind (_resultpos_x_4 _resultpos_y_2) (`KismetMathLibrary.BreakVector2D` (`local.ResultPos`)))
  (bind _deadzone_x_7 (`KismetMathLibrary.BreakVector2D` (`local.DeadZone`)))
  (bind (_deadzone_x_8 _deadzone_y_4) (`KismetMathLibrary.BreakVector2D` (`local.DeadZone`)))
  (set `local.ResultPos` ScreenPos)
  ;[1 1 1] < deadzone X
  (if (< _screenpos_x _deadzone_x_2)
    (set `local.ResultPos` (`KismetMathLibrary.MakeVector2D` _deadzone_x_5 _resultpos_y_2))
    (set `local.bIsOutBounds` true))
  ;[1 1 1] > deadzone X
  (if (> _screenpos_x_2 (- 1.0 _deadzone_x_6))
    (set `local.ResultPos` (`KismetMathLibrary.MakeVector2D` (- 1.0 _deadzone_x_7) _resultpos_y))
    (set `local.bIsOutBounds` true))
  ;[1 1 1] < deadzone Y
  (if (< _screenpos_y _deadzone_y_4)
    (set `local.ResultPos` (`KismetMathLibrary.MakeVector2D` _resultpos_x _deadzone_y_2))
    (set `local.bIsOutBounds` true))
  ;[1 1 1] > deadzone Y
  (if (> _screenpos_y_2 (- 1.0 _deadzone_y_3))
    (set `local.ResultPos` (`KismetMathLibrary.MakeVector2D` _resultpos_x_2 (- 1.0 _deadzone_y)))
    (set `local.bIsOutBounds` true))
  (return (`local.bIsOutBounds`) (`local.ResultPos`)))

(fn `UserConstructionScript`)