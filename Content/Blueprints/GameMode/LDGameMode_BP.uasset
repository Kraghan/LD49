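; Game mode for mixer-based levels that times the run and shows the level-done screen.
; On BeginPlay it finds the Mixer_BP actor, binds to its good-ingredient event and starts the timer in game-only input, or switches to UI input with a cursor if none exists.
; When a good ingredient fills the mixer, it prints the elapsed time and opens LevelDone_Widget with the mixer's next-level reference and time-based score.
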(event `self.ReceiveBeginPlay`
  (bind _returnvalue (`GameplayStatics.GetPlayerController` 0))
  (bind _returnvalue_2 (`GameplayStatics.GetPlayerController` 0))
  (bind _returnvalue_3 (`GameplayStatics.GetActorOfClass` "/Game/Blueprints/LevelDesign/Mixer_BP.Mixer_BP_C"))
  (`/Engine/EditorBlueprintResources/StandardMacros.IsValid` _returnvalue_3
    (:`Is Valid`
      (bind _output_get (set `self.Mixer` _returnvalue_3))
      (add `/Game/Blueprints/LevelDesign/Mixer_BP.OnGoodIngredient` _output_get (delegate `OnGoodIngredient`))
      (`WidgetBlueprintLibrary.SetInputMode_GameOnly` _returnvalue_2)
      (set `PlayerController.bShowMouseCursor` false _returnvalue_2)
      (set `self.StartTime` (`GameplayStatics.GetRealTimeSeconds`)))
    (:`Is Not Valid`
      (`WidgetBlueprintLibrary.SetInputMode_UIOnlyEx` _returnvalue null)
      (set `PlayerController.bShowMouseCursor` true _returnvalue))))

(event `OnGoodIngredient`
  (params (IngredientAdded :type "/Game/Blueprints/Interactions/Ingredients_BP Class Reference"))
  (bind _returnvalue (`GameplayStatics.GetPlayerController` 0))
  (bind _returnvalue_2 (- (`GameplayStatics.GetRealTimeSeconds`) (`self.StartTime`)))
  (if (`/Game/Blueprints/LevelDesign/Mixer_BP.IsFull` (`self.Mixer`))
    (`KismetSystemLibrary.PrintString` (`KismetStringLibrary.Concat_StrStr` "Level done in : " (`KismetStringLibrary.Conv_DoubleToString` _returnvalue_2) " seconds !") true true (struct :`R` 1.0 :`A` 1.0) 5.0)
    ;[1 1 1] Show menu
    (bind _returnvalue_3 (`|CreateWidget` "/Game/Blueprints/UI/LevelDone_Widget.LevelDone_Widget_C" _returnvalue (`/Game/Blueprints/LevelDesign/Mixer_BP.NextLevelRef` (`self.Mixer`)) (`/Game/Blueprints/LevelDesign/Mixer_BP.GetScoreTime` (`self.Mixer`) _returnvalue_2)))
    (`UserWidget.AddToViewport` _returnvalue_3 0)
    (`WidgetBlueprintLibrary.SetInputMode_UIOnlyEx` _returnvalue _returnvalue_3)
    (set `PlayerController.bShowMouseCursor` true _returnvalue)))

(fn `UserConstructionScript`)