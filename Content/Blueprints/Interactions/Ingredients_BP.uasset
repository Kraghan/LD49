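; Interactable ingredient actor that a player picks up, allowed only while that player's hands are empty.
; Interact passes the player to ChangeOwner, which casts the new owner to ObjectHolder and hands itself over through SetObject.
; It then tells any valid previous owner to clear its object and records the new holder as OwningActor, so ingredients transfer between holders.
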(event `/Game/Blueprints/Interactions/Interactible.Interact`
  (params (Player :type "/Game/Blueprints/Character/Character_BP Object Reference"))
  (`self.ChangeOwner` Player))

(fn `CanInteract`
  (params (Player :type "/Game/Blueprints/Character/Character_BP Object Reference"))
  (returns (CanInteract :type Boolean))
  (return (not (`/Game/Blueprints/Character/Character_BP.HasSomethingInHands` Player))))

(fn `ChangeOwner`
  (params (NewOwner :type "Actor Object Reference"))
  (bind _asobject_holder (cast `/Game/Blueprints/ObjectHolder` NewOwner))
  (`/Game/Blueprints/ObjectHolder.SetObject` _asobject_holder self)
  (`/Engine/EditorBlueprintResources/StandardMacros.IsValid` (`self.OwningActor`)
    (:`Is Valid`
      (message `/Game/Blueprints/ObjectHolder.ClearObject` (`self.OwningActor`)))
    (:`Is Not Valid`
      _))
  (set `self.OwningActor` (`local.NewOwner`)))

(fn `UserConstructionScript`)