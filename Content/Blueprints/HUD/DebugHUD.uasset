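; DebugHUD is a HUD Blueprint for visualizing camera dead zones and target positions, though DrawHUD currently only calls its parent.
; Disconnected graphs read LDCameraManager_BP to draw hard and soft dead zones and mark and print FinalPos.
; Another disconnected graph marks the projected Character_BP location on screen.
; DrawDeadZone shades four screen-edge bands, sized as fractions of screen width and height.
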(event `self.ReceiveTick`
  (params (DeltaSeconds :type "Float (single-precision)")))

(event `self.ReceiveDrawHUD`
  (params (SizeX :type Integer) (SizeY :type Integer))
  (`parent.ReceiveDrawHUD` SizeX SizeY))

(fn `Draw Dead Zone`
  (params (DeadzoneSize :type "Vector2D Structure") (ScreenSizeX :type Integer) (ScreenSizeY :type Integer) (Color :type "LinearColor Structure"))
  (bind _returnvalue (`KismetMathLibrary.Conv_IntToDouble` ScreenSizeY))
  (bind _returnvalue_2 (`KismetMathLibrary.Conv_IntToDouble` ScreenSizeX))
  (bind (_deadzonesize_x _deadzonesize_y) (`KismetMathLibrary.BreakVector2D` (`local.DeadzoneSize`)))
  (bind _deadzonesize_x_2 (`KismetMathLibrary.BreakVector2D` (`local.DeadzoneSize`)))
  (bind _returnvalue_3 (* ScreenSizeX _deadzonesize_x_2))
  (bind _returnvalue_4 (* ScreenSizeY _deadzonesize_y))
  (`|ExecutionSequence`
    (:`then_0`
      (`self.DrawRect` Color 0.0 0.0 _returnvalue_3 _returnvalue)
      (`self.DrawRect` Color (- (`KismetMathLibrary.Conv_IntToDouble` ScreenSizeX) _returnvalue_3) 0.0 _returnvalue_3 _returnvalue))
    (:`then_1`
      (`self.DrawRect` Color 0.0 0.0 _returnvalue_2 _returnvalue_4)
      (`self.DrawRect` Color 0.0 (- (`KismetMathLibrary.Conv_IntToDouble` ScreenSizeY) _returnvalue_4) _returnvalue_2 _returnvalue_4))))

(fn `UserConstructionScript`)